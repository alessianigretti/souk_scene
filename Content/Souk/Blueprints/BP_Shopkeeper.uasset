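; BP_Shopkeeper is a souk shopkeeper that tracks a customer through AI perception.
; On BeginPlay it picks a random skeletal mesh, stores its starting location as home and assigns itself to its Shop.
; When perception updates and it has no valid target, it takes the first updated actor if that is a BP_Customer.
; It clears that target when perception reports a target forgotten.
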(event OnPerceptionUpdated(AIPerception)
  (params (UpdatedActors :type Array%20of%20Actor%20Object%20References))
  (Utilities|IsValid (Variables|Default|GetTargetCustomer)
    (:Is%20Not%20Valid
      (bind _asbp_customer (Utilities|Casting|CastToBP_Customer (Utilities|Array|Get(acopy) UpdatedActors)))
      (Variables|Default|SetTargetCustomer _asbp_customer))))

(event OnTargetPerceptionForgotten(AIPerception)
  (params (Actor :type Actor%20Object%20Reference))
  (Variables|Default|SetTargetCustomer 0))

(event EventBeginPlay
  (Components|SkeletalMesh|SetSkeletalMeshAsset (Variables|Character|GetMesh) (.OutItem (Utilities|Array|Random (Variables|Default|GetSkeletalMeshes))))
  (Variables|Default|SetHomeLocation (Transformation|GetActorLocation))
  (Default|AssignShopkeeper (Variables|Default|GetShop) self))

(fn ConstructionScript)