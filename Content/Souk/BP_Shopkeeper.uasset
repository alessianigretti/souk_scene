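; BP_Shopkeeper is a shopkeeper that watches for a character in front of it.
; Every tick it sphere-traces for Pawns along a short stretch ahead, offset forward and upward from its location.
; A Character hit becomes Target and sets NeckRotationYaw from the look-at yaw plus a half turn, presumably for head-turn animation.
; When nothing is hit, the yaw resets to zero and Target clears.
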(event EventTick
  (params (DeltaSeconds :type Float%20%28single-precision%29))
  (bind _returnvalue (Transformation|GetActorLocation))
  (bind _returnvalue_2 (Transformation|GetActorUpVector))
  (bind _returnvalue_3 (Transformation|GetActorForwardVector))
  (bind _returnvalue_4 (* _returnvalue_3 1.5e+02))
  (bind _returnvalue_5 (* _returnvalue_2 5e+01))
  (bind _returnvalue_6 (+ _returnvalue _returnvalue_4 _returnvalue_5))
  (bind (_outhit _returnvalue_7) (Collision|SphereTraceForObjects _returnvalue_6 (+ _returnvalue_6 (* (Transformation|GetActorForwardVector) 2e+02)) 1e+02 (Utilities|Array|MakeArray "ObjectTypeQuery3") false 0 "None"))
  (if _returnvalue_7
    (bind _ascharacter (Utilities|Casting|CastToCharacter (.HitActor (Collision|BreakHitResult _outhit))))
    (Variables|Default|SetTarget _ascharacter)
    (Variables|Default|SetNeckRotationYaw (+ (.Yaw (Math|Rotator|BreakRotator (Math|Rotator|FindLookatRotation (Transformation|GetActorLocation) (Transformation|GetActorLocation _ascharacter)))) 1.8e+02))
    (else
      (Variables|Default|SetNeckRotationYaw 0.0)
      (Variables|Default|SetTarget 0))))

(fn ConstructionScript)